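; BP_HeatLamp is a heat lamp with a trigger sphere that forces the cold potato to drop after time under it.
; BeginPlay caches the first ColdPotato_BP, whose overlap plays the TimeInLamp timeline.
; Timeline Finished calls DropPotato with the potato's parent actor and prints that actor's name.
; End overlap compares PotatoRef to itself, so any actor leaving reverses the timeline, which can also fire Finished.
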(event OnComponentBeginOverlap(Sphere)
  (params (OverlappedComponent :type Primitive%20Component%20Object%20Reference) (OtherActor :type Actor%20Object%20Reference) (OtherComp :type Primitive%20Component%20Object%20Reference) (OtherBodyIndex :type Integer) (bFromSweep :type Boolean) (SweepResult :type Hit%20Result%20Structure%20%28by%20ref%29))
  (bind _potato_ref (Variables|Default|GetPotato%20Ref))
  (bind _parentactor (Variables|/Game/ColdPotato_BP.ColdPotato_BP_C|GetParentActor _potato_ref))
  (if (== OtherActor (Variables|Default|GetPotato%20Ref))
    (Timeline|TimeInLamp Play
      (:Finished
        (Default|DropPotato _potato_ref _parentactor)
        (Development|PrintString (Utilities|GetDisplayName _parentactor))))))

(event OnComponentEndOverlap(Sphere)
  (params (OverlappedComponent :type Primitive%20Component%20Object%20Reference) (OtherActor :type Actor%20Object%20Reference) (OtherComp :type Primitive%20Component%20Object%20Reference) (OtherBodyIndex :type Integer))
  (bind _potato_ref (Variables|Default|GetPotato%20Ref))
  (bind _potato_ref_2 (Variables|Default|GetPotato%20Ref))
  (bind _parentactor (Variables|/Game/ColdPotato_BP.ColdPotato_BP_C|GetParentActor _potato_ref_2))
  (if (== _potato_ref _potato_ref)
    (Timeline|TimeInLamp Reverse
      (:Finished
        (Default|DropPotato _potato_ref_2 _parentactor)
        (Development|PrintString (Utilities|GetDisplayName _parentactor))))))

(event EventBeginPlay
  (bind _outactors (Actor|GetAllActorsOfClass "/Game/ColdPotato_BP.ColdPotato_BP_C"))
  (Variables|Default|SetPotato%20Ref (Utilities|Array|Get(acopy) _outactors)))

(fn ConstructionScript)