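; Heat lamp hazard actor that spawns at a random reachable navmesh point, retrying if placement fails, with its spotlight dark.
; GetPotatoActor, not called within this graph, caches the ColdPotato_BP actor and fades the light in by timeline.
; Roaming between random navmesh points and dropping the potato after timed exposure are present but disconnected, leaving MoveHeatLamp and the overlap events without effect.
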(event OnComponentBeginOverlap(CollisionSphere)
  (params (OverlappedComponent :type Primitive%20Component%20Object%20Reference) (OtherActor :type Actor%20Object%20Reference) (OtherComp :type Primitive%20Component%20Object%20Reference) (OtherBodyIndex :type Integer) (bFromSweep :type Boolean) (SweepResult :type Hit%20Result%20Structure%20%28by%20ref%29))
  ;[0.15 0.15 0.15 0.5] Sphere Collision (2 Seconds (Timeline) to Drop Potato)
)

(event OnComponentEndOverlap(CollisionSphere)
  (params (OverlappedComponent :type Primitive%20Component%20Object%20Reference) (OtherActor :type Actor%20Object%20Reference) (OtherComp :type Primitive%20Component%20Object%20Reference) (OtherBodyIndex :type Integer))
  ;[0.15 0.15 0.15 0.5] Sphere Collision (2 Seconds (Timeline) to Drop Potato)
)

(event OnComponentBeginOverlap(NearHeatLamp)
  (params (OverlappedComponent :type Primitive%20Component%20Object%20Reference) (OtherActor :type Actor%20Object%20Reference) (OtherComp :type Primitive%20Component%20Object%20Reference) (OtherBodyIndex :type Integer) (bFromSweep :type Boolean) (SweepResult :type Hit%20Result%20Structure%20%28by%20ref%29))
  (if (Actor|ActorHasTag OtherActor "NPC")
    _))

(event OnComponentEndOverlap(NearHeatLamp)
  (params (OverlappedComponent :type Primitive%20Component%20Object%20Reference) (OtherActor :type Actor%20Object%20Reference) (OtherComp :type Primitive%20Component%20Object%20Reference) (OtherBodyIndex :type Integer))
  (if (Actor|ActorHasTag OtherActor "NPC")
    _))

(event Custom|MoveHeatLamp
  ;[0.15 0.15 0.15 0.5] Move Heat Lamp
)

(event Custom|Get%20Potato%20Actor
  ;[0.15 0.15 0.15 0.5] Get Potato Ref
  (bind _outactors (Actor|GetAllActorsOfClass "/Game/04_Blueprints/ColdPotato_BP.ColdPotato_BP_C"))
  (Variables|Default|SetPotato%20Ref (Utilities|Array|Get(acopy) _outactors))
  (CallFunction|StartHeatLamp))

(event Custom|Start%20Heat%20Lamp
  ;[0.15 0.15 0.15 0.5] Fade Head Lamp In
  (bind _lerp_ (Timeline|HeatLampBrightness Play)
    (:Update
      (Rendering|Components|Light|SetIntensity (Variables|Default|GetSpotLight) (Math|Float|Lerp 0.0 (Variables|Default|GetHeatLampItensity) _lerp_)))
    (:Finished
      (CallFunction|MoveHeatLamp))))

(event Custom|FindSpawnPoint
  (bind _returnvalue (Transformation|GetActorLocation))
  (bind _randomlocation (AI|Navigation|GetRandomReachablePointinRadius _returnvalue 1e+03 0 0))
  (bind (_x _y) (Math|Vector|BreakVector _randomlocation))
  ;[0.15 0.15 0.15 0.5] Random Spawn Point in Navigable Area
  (bind _returnvalue_2 (Transformation|SetActorLocation (Math|Vector|MakeVector _x _y (.Z (Math|Vector|BreakVector _returnvalue))) false false))
  (if (not _returnvalue_2)
    (CallFunction|FindSpawnPoint)))

(event EventBeginPlay
  (bind _returnvalue (Transformation|GetActorLocation))
  (bind _spotlight (Variables|Default|GetSpotLight))
  (bind _randomlocation (AI|Navigation|GetRandomReachablePointinRadius _returnvalue 1e+03 0 0))
  (bind (_x _y) (Math|Vector|BreakVector _randomlocation))
  ;[0.15 0.15 0.15 0.5] Set Light Intensity
  (Variables|Default|SetHeatLampItensity (Variables|/Script/Engine.LightComponentBase|GetIntensity _spotlight))
  (Rendering|Components|Light|SetIntensity _spotlight 0.0)
  ;[0.15 0.15 0.15 0.5] Random Spawn Point in Navigable Area
  (bind _returnvalue_2 (Transformation|SetActorLocation (Math|Vector|MakeVector _x _y (.Z (Math|Vector|BreakVector _returnvalue))) false false))
  (if (not _returnvalue_2)
    (CallFunction|FindSpawnPoint)))

(fn ConstructionScript)