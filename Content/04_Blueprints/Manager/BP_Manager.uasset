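; Match manager for the potato game that sets up the round and records playtest telemetry.
; On BeginPlay it loads the save, adds the timer HUD, spawns three AI rivals and recursively moves all players to random unique spawn points.
; A Tick countdown spawns the potato and notifies player, heat lamps and AI controllers.
; HeatMapScreenshots captures per-role telemetry heatmaps via console command, writes a results text file and increments saved games played.
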(event Custom|Move%20Actors%20to%20Spawn%20Points
  (bind _players (Variables|Default|GetPlayers))
  (bind _playerindex (Variables|Default|GetPlayerIndex))
  (bind _spawnpoints (Variables|Default|GetSpawnPoints))
  (bind _output (Utilities|Array|Get(acopy) _players _playerindex))
  ;[0.15 0.15 0.15 0.5] Spawn Players
  (bind _output_get (Variables|Default|SetCurrent%20Spawn%20Point (Utilities|Array|Get(acopy) _spawnpoints (Math|Random|RandomIntegerinRange 0 (Utilities|Array|LastIndex _spawnpoints)))))
  (Utilities|IsValid _output_get
    (:Is%20Valid
      (Utilities|IsValid _output
        (:Is%20Valid
          (Transformation|SetActorLocationAndRotation _output (.location (Transformation|GetWorldTransform (Variables|/Script/Engine.Actor|GetRootComponent (Variables|Default|GetCurrent%20Spawn%20Point)))) (.rotation (Transformation|GetWorldTransform (Variables|/Script/Engine.Actor|GetRootComponent (Variables|Default|GetCurrent%20Spawn%20Point)))))
          (if (Actor|ActorHasTag _output "Player")
            (bind _asbp_first_person_character (Utilities|Casting|CastToBP_FirstPersonCharacter _output))
            (Pawn|SetControlRotation (Game|GetPlayerController 0) (Math|Rotator|FindLookatRotation (Transformation|GetWorldLocation (Variables|/Script/Engine.Character|GetCapsuleComponent _asbp_first_person_character)) (Transformation|GetWorldLocation (Variables|/Game/04_Blueprints/PlayerSpawning/BP_PlayerSpawnPoint.BP_PlayerSpawnPoint_C|GetArrow (Variables|Default|GetCurrent%20Spawn%20Point))))))
          (Utilities|Array|RemoveItem (Variables|Default|GetSpawnPoints) (Variables|Default|GetCurrent%20Spawn%20Point))
          (Math|Integer|IncrementInt (Variables|Default|GetPlayerIndex)
            (:%20%20
              (CallFunction|MoveActorstoSpawnPoints))))))
    (:Is%20Not%20Valid
      (Utilities|FlowControl|Delay 0.1)
      (CallFunction|MoveActorstoSpawnPoints))))

(event Custom|Get%20Players
  ;[0.15 0.15 0.15 0.5] Get Players
  (CallFunction|SpawnPlayers(Actors))
  (CallFunction|MoveActorstoSpawnPoints))

(event Custom|Screenshots
  (Variables|Default|SetNickname (Variables|/Game/04_Blueprints/BP_PotatoSaveGame.BP_PotatoSaveGame_C|GetNickname (Variables|Default|GetSave%20Game%20Ref)))
  (Utilities|FlowControl|Delay 0.1)
  (Default|HeatMapAllView (Variables|Default|GetTelemetry%20REF))
  (CallFunction|ScreenshotHeatMap (Utilities|String|ToString(Text) (Utilities|Text|FormatText "{Nickname}_HeatMap_All" (Variables|Default|GetNickname))))
  (Utilities|FlowControl|Delay 0.1)
  (Default|HeatMapPlayer (Variables|Default|GetTelemetry%20REF))
  (CallFunction|ScreenshotHeatMap (Utilities|String|ToString(Text) (Utilities|Text|FormatText "{Nickname}_HeatMap_Player" (Variables|Default|GetNickname))))
  (Utilities|FlowControl|Delay 0.1)
  (Default|HeatMapHoarder (Variables|Default|GetTelemetry%20REF))
  (CallFunction|ScreenshotHeatMap (Utilities|String|ToString(Text) (Utilities|Text|FormatText "{Nickname}_HeatMap_Hoarder" (Variables|Default|GetNickname))))
  (Utilities|FlowControl|Delay 0.1)
  (Default|HeatMapIntrceptor (Variables|Default|GetTelemetry%20REF))
  (CallFunction|ScreenshotHeatMap (Utilities|String|ToString(Text) (Utilities|Text|FormatText "{Nickname}_HeatMap_Interceptor" (Variables|Default|GetNickname))))
  (Utilities|FlowControl|Delay 0.1)
  (Default|HeatMapOppertunist (Variables|Default|GetTelemetry%20REF))
  (CallFunction|ScreenshotHeatMap (Utilities|String|ToString(Text) (Utilities|Text|FormatText "{Nickname}_HeatMap_Opportunist" (Variables|Default|GetNickname))))
  (CallFunction|CreateTextFileandUpdateSaveGame))

(event Custom|GetSaveGame
  (bind _returnvalue (SaveGame|DoesSaveGameExist "PotatoSave"))
  (if _returnvalue
    (bind _returnvalue_2 (SaveGame|LoadGamefromSlot "PotatoSave"))
    (bind _asbp_potato_save_game (Utilities|Casting|CastToBP_PotatoSaveGame _returnvalue_2))
    (Variables|Default|SetSave%20Game%20Ref _asbp_potato_save_game)
    (else
      (Development|PrintString "NoSaveGameFound"))))

(event EventBeginPlay
  ;[0.15 0.15 0.15 0.5] Begin Play, Get Spawn Points
  (CallFunction|GetSpawnPointsandCreateGameHUD)
  (CallFunction|GetSaveGame))

(event EventTick
  (params (DeltaSeconds :type Float%20%28single-precision%29))
  ;[0.15 0.15 0.15 0.5] Temp Timer
  (if (<= (Variables|Default|GetTime%20to%20Spawn%20Potato) 0.0)
    (Utilities|FlowControl|DoOnce false
      (:Completed
        (CallFunction|SpawnPotato(Actor))))
    (else
      (Variables|Default|SetTime%20to%20Spawn%20Potato (- (Variables|Default|GetTime%20to%20Spawn%20Potato) DeltaSeconds)))))

(fn ConstructionScript)

(fn SpawnPlayers(Actors)
  (bind _asbp_first_person_character (Utilities|Casting|CastToBP_FirstPersonCharacter (Game|GetPlayerCharacter 0)))
  (Utilities|Array|Add (Variables|Default|GetPlayers) _asbp_first_person_character)
  (bind _returnvalue (Game|SpawnActorfromClass "/Game/03_AI-Enemies/Characters/Hoarder/BP_AI_Hoarder.BP_AI_Hoarder_C" (Math|Transform|MakeTransform "0, 0, 0" "0, 0, 0" "1.000000,1.000000,1.000000") "AlwaysSpawn" "MultiplyWithRoot" 0 "/Game/06_Assets/AssetPacks/Enemy_AI_Models/M_Player_Hoarder.M_Player_Hoarder" 0))
  (Utilities|Array|Add (Variables|Default|GetPlayers) _returnvalue)
  (bind _returnvalue_2 (Game|SpawnActorfromClass "/Game/03_AI-Enemies/Characters/Interceptor/BP_AI_Interceptor.BP_AI_Interceptor_C" (Math|Transform|MakeTransform "0, 0, 0" "0, 0, 0" "1.000000,1.000000,1.000000") "AlwaysSpawn" "MultiplyWithRoot" 0 "/Game/06_Assets/AssetPacks/Enemy_AI_Models/M_Player_Interceptor.M_Player_Interceptor" 0))
  (Utilities|Array|Add (Variables|Default|GetPlayers) _returnvalue_2)
  (bind _returnvalue_3 (Game|SpawnActorfromClass "/Game/03_AI-Enemies/Characters/Oppertunist/BP_AI_Oppertunist.BP_AI_Oppertunist_C" (Math|Transform|MakeTransform "0, 0, 0" "0, 0, 0" "1.000000,1.000000,1.000000") "AlwaysSpawn" "MultiplyWithRoot" 0 "/Game/06_Assets/AssetPacks/Enemy_AI_Models/M_Player_Oppertunist.M_Player_Oppertunist" 0))
  (Utilities|Array|Add (Variables|Default|GetPlayers) _returnvalue_3))

(fn SpawnPotato(Actor)
  (bind _outactors (Actor|GetAllActorsOfClass "/Game/04_Blueprints/PlayerSpawning/BP_PotatoSpawnPoint.BP_PotatoSpawnPoint_C"))
  (bind _returnvalue (Game|SpawnActorfromClass "/Game/04_Blueprints/ColdPotato_BP.ColdPotato_BP_C" (Math|Transform|MakeTransform (Transformation|GetWorldLocation (Variables|/Game/04_Blueprints/PlayerSpawning/BP_PotatoSpawnPoint.BP_PotatoSpawnPoint_C|GetSphere (Utilities|Array|Get(acopy) _outactors (Math|Random|RandomIntegerinRange 0 (Utilities|Array|LastIndex _outactors))))) "0, 0, 0" "1.000000,1.000000,1.000000") "AlwaysSpawn" "MultiplyWithRoot" 0 0))
  (Utilities|FlowControl|Sequence
    (:then_0
      (bind _asbp_first_person_character (Utilities|Casting|CastToBP_FirstPersonCharacter (Game|GetPlayerCharacter 0)))
      (Default|GetPotatoRef _asbp_first_person_character)
      (bind _outactors_2 (Actor|GetAllActorsOfClass "/Game/04_Blueprints/HeatLamp/BP_HeatLamp.BP_HeatLamp_C"))
      (for _array_element _outactors_2
        (Default|GetPotatoActor _array_element)))
    (:then_1
      (bind _outactors_3 (Actor|GetAllActorsOfClass "/Game/03_AI-Enemies/AI_Parent_ControllerClass.AI_Parent_ControllerClass_C"))
      (for _array_element_2 _outactors_3
        (Default|StartGameBBKey _array_element_2 _returnvalue)))))

(fn GetSpawnPointsandCreateGameHUD
  (bind _outactors (Actor|GetAllActorsOfClass "/Game/04_Blueprints/PlayerSpawning/BP_PlayerSpawnPoint.BP_PlayerSpawnPoint_C"))
  (Variables|Default|SetSpawnPoints _outactors)
  (CallFunction|GetPlayers)
  (bind _returnvalue (UserInterface|CreateWidget "/Game/05_UserInterface/Gameplay/WB_Timer.WB_Timer_C"))
  (UserInterface|Viewport|AddtoViewport _returnvalue 0))

(fn HeatMapScreenshots
  (params (Timer%20Ref :type WB%20Timer%20Object%20Reference))
  (Variables|Default|SetTimer%20REF Timer%20Ref)
  (bind _returnvalue (Actor|GetActorOfClass "/Game/04_Blueprints/Telemetry/BP_Telemetry.BP_Telemetry_C"))
  (bind _output_get (Variables|Default|SetTelemetry%20REF _returnvalue))
  (Default|HideorShowTelemetry _output_get)
  (Default|HideAll _output_get)
  (CallFunction|Screenshots))

(fn CreateTextFileandUpdateSaveGame
  (bind _timer_ref (Variables|Default|GetTimer%20REF))
  (bind _save_game_ref (Variables|Default|GetSave%20Game%20Ref))
  (switch int (Variables|/Game/04_Blueprints/BP_PotatoSaveGame.BP_PotatoSaveGame_C|GetDifficultySetting (Variables|Default|GetSave%20Game%20Ref))
    (:0
      (Variables|Default|SetDfficultyText "Easy"))
    (:1
      (Variables|Default|SetDfficultyText "Medium"))
    (:2
      (Variables|Default|SetDfficultyText "Hard")))
  (Class|VictoryBPFunctionLibrary|FileIOSaveStringTexttoFile (Utilities|String|ToString(Text) (Utilities|Text|FormatText "{FilePath}/Saved/Screenshots/WindowsEditor" (Class|KismetSystemLibrary|GetProjectDirectory))) (Utilities|String|ToString(Text) (Utilities|Text|FormatText "{GamePlayedNum}_{Nickname}_Info" (Variables|/Game/04_Blueprints/BP_PotatoSaveGame.BP_PotatoSaveGame_C|GetGamesPlayed (Variables|Default|GetSave%20Game%20Ref)) (Variables|Default|GetNickname))) (Utilities|String|ToString(Text) (Utilities|Text|FormatText "Playtester Nickname: {Nickname} 
 
Who Won: {WhoWon} 
 
Difficulty Option: {DifficultyOption} 
 
Time Held on Each Player: 
Player: {Player_TimeHeld} 
Hoarder: {Hoarder_TimeHeld} 
Interceptor: {Interceptor_TimeHeld} 
Opportunist: {Opportunist_TimeHeld}" (Variables|Default|GetNickname) (Variables|/Script/UMG.TextBlock|GetText (Variables|/Game/05_UserInterface/Gameplay/WB_Timer.WB_Timer_C|GetWhoWonTxT _timer_ref)) (Variables|Default|GetDfficultyText) (Variables|/Script/UMG.TextBlock|GetText (Variables|/Game/05_UserInterface/Gameplay/WB_Timer.WB_Timer_C|GetPlayer_01_TIMEHELD _timer_ref)) (Variables|/Script/UMG.TextBlock|GetText (Variables|/Game/05_UserInterface/Gameplay/WB_Timer.WB_Timer_C|GetPlayer_02_TIMEHELD _timer_ref)) (Variables|/Script/UMG.TextBlock|GetText (Variables|/Game/05_UserInterface/Gameplay/WB_Timer.WB_Timer_C|GetPlayer_03_TIMEHELD _timer_ref)) (Variables|/Script/UMG.TextBlock|GetText (Variables|/Game/05_UserInterface/Gameplay/WB_Timer.WB_Timer_C|GetPlayer_04_TIMEHELD _timer_ref)))) false false)
  (bind _result (Math|Integer|IncrementInt (Variables|/Game/04_Blueprints/BP_PotatoSaveGame.BP_PotatoSaveGame_C|GetGamesPlayed _save_game_ref))
    (:%20%20
      (Variables|/Game/04_Blueprints/BP_PotatoSaveGame.BP_PotatoSaveGame_C|SetGamesPlayed _save_game_ref _result)
      (SaveGame|SaveGametoSlot (Variables|Default|GetSave%20Game%20Ref) "PotatoSave"))))

(fn ScreenshotHeatMap
  (params (FileName :type String))
  (bind _output_get (Variables|Default|SetScreenshot%20Command (Utilities|Text|FormatText "{HighResShot_Cmd} filename={FileName}" (Variables|Default|GetHighResShot_Command) (Utilities|String|ToString(Text) (Utilities|Text|FormatText "{GameNumber}_{FileName}" (Variables|/Game/04_Blueprints/BP_PotatoSaveGame.BP_PotatoSaveGame_C|GetGamesPlayed (Variables|Default|GetSave%20Game%20Ref)) FileName)))))
  (Development|ExecuteConsoleCommand (Utilities|String|ToString(Text) _output_get) (Game|GetPlayerController (Variables|/Script/Engine.Pawn|GetPlayerState (Game|GetPlayerCharacter 0)))))