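; Game manager that sets up a hot-potato style match with the player, three AI opponents and a timer widget.
; On BeginPlay it gathers spawn points, spawns the AI and recursively teleports everyone to random points, though the removed point is re-rolled separately from the one used.
; It also picks a random potato location.
; Tick counts down, then spawns the potato once, starts its gameplay bools and notifies the first heat lamp.
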(event Custom|Spawn%20Players
  (bind _playerindex (Variables|Default|GetPlayerIndex))
  (bind _players (Variables|Default|GetPlayers))
  (bind _spawnpoints (Variables|Default|GetSpawnPoints))
  (bind _returnvalue (Utilities|Array|LastIndex _spawnpoints))
  (bind _output (Utilities|Array|Get(acopy) _players _playerindex))
  (bind _returnvalue_2 (Math|Random|RandomIntegerinRange 0 _returnvalue))
  (bind _output_2 (Utilities|Array|Get(acopy) _spawnpoints _returnvalue_2))
  ;[0.15 0.15 0.15 0.5] Spawn Players
  (Utilities|IsValid _output
    (:Is%20Valid
      (Transformation|SetActorLocation _output (Transformation|GetWorldLocation (Variables|/Game/04_Blueprints/PlayerSpawning/BP_PlayerSpawnPoint.BP_PlayerSpawnPoint_C|GetCube _output_2)) false true)
      (Utilities|Array|RemoveItem (Variables|Default|GetSpawnPoints) _output_2)
      (Math|Integer|IncrementInt (Variables|Default|GetPlayerIndex)
        (:%20%20
          (CallFunction|SpawnPlayers))))))

(event Custom|Get%20Players
  ;[0.15 0.15 0.15 0.5] Get Players
  (bind _asbp_first_person_character (Utilities|Casting|CastToBP_FirstPersonCharacter (Game|GetPlayerCharacter 0)))
  (Utilities|Array|Add (Variables|Default|GetPlayers) _asbp_first_person_character)
  (bind _returnvalue (Game|SpawnActorfromClass "/Game/03_AI-Enemies/Hoarder/BP_AI_Hoarder.BP_AI_Hoarder_C" (Math|Transform|MakeTransform "0, 0, 0" "0, 0, 0" "1.000000,1.000000,1.000000") "Undefined" "MultiplyWithRoot" 0 0))
  (Utilities|Array|Add (Variables|Default|GetPlayers) _returnvalue)
  (bind _returnvalue_2 (Game|SpawnActorfromClass "/Game/03_AI-Enemies/Interceptor/BP_AI_Interceptor.BP_AI_Interceptor_C" (Math|Transform|MakeTransform "0, 0, 0" "0, 0, 0" "1.000000,1.000000,1.000000") "Undefined" "MultiplyWithRoot" 0 0))
  (Utilities|Array|Add (Variables|Default|GetPlayers) _returnvalue_2)
  (bind _returnvalue_3 (Game|SpawnActorfromClass "/Game/03_AI-Enemies/Oppertunist/BP_AI_Oppertunist.BP_AI_Oppertunist_C" (Math|Transform|MakeTransform "0, 0, 0" "0, 0, 0" "1.000000,1.000000,1.000000") "Undefined" "MultiplyWithRoot" 0 0))
  (Utilities|Array|Add (Variables|Default|GetPlayers) _returnvalue_3)
  (CallFunction|SpawnPlayers))

(event Custom|Spawn%20Potato
  ;[0.15 0.15 0.15 0.5] Spawn Potato
  (bind _returnvalue (Game|SpawnActorfromClass "/Game/04_Blueprints/ColdPotato_BP.ColdPotato_BP_C" (Math|Transform|MakeTransform (Variables|Default|GetPotatoSpawnLocation) "0, 0, 0" "1.000000,1.000000,1.000000") "AlwaysSpawn" "MultiplyWithRoot" 0 0))
  (Default|StartGamePlayerBools _returnvalue)
  (bind _outactors (Actor|GetAllActorsOfClass "/Game/04_Blueprints/HeatLamp/BP_HeatLamp.BP_HeatLamp_C"))
  (Default|GetPotatoActor (Utilities|Array|Get(acopy) _outactors)))

(event Custom|Get%20Random%20Potato%20Spawn%20Point
  ;[0.15 0.15 0.15 0.5] Get Random Potato Spawn Point
  (bind _outactors (Actor|GetAllActorsOfClass "/Game/04_Blueprints/PlayerSpawning/BP_PotatoSpawnPoint.BP_PotatoSpawnPoint_C"))
  (Variables|Default|SetPotatoSpawnLocation (Transformation|GetWorldLocation (Variables|/Game/04_Blueprints/PlayerSpawning/BP_PotatoSpawnPoint.BP_PotatoSpawnPoint_C|GetSphere (Utilities|Array|Get(acopy) _outactors (Math|Random|RandomIntegerinRange 0 (Utilities|Array|LastIndex _outactors)))))))

(event EventBeginPlay
  ;[0.15 0.15 0.15 0.5] Get Spawn Points
  (bind _outactors (Actor|GetAllActorsOfClass "/Game/04_Blueprints/PlayerSpawning/BP_PlayerSpawnPoint.BP_PlayerSpawnPoint_C"))
  (Variables|Default|SetSpawnPoints _outactors)
  (CallFunction|GetPlayers)
  (CallFunction|GetRandomPotatoSpawnPoint)
  (bind _returnvalue (UserInterface|CreateWidget "/Game/05_UserInterface/WB_Timer.WB_Timer_C"))
  (UserInterface|Viewport|AddtoViewport _returnvalue 0))

(event EventTick
  (params (DeltaSeconds :type Float%20%28single-precision%29))
  ;[0.15 0.15 0.15 0.5] Temp Timer
  (if (<= (Variables|Default|GetTime%20to%20Spawn%20Potato) 0.0)
    (Utilities|FlowControl|DoOnce false
      (:Completed
        (CallFunction|SpawnPotato)))
    (else
      (Variables|Default|SetTime%20to%20Spawn%20Potato (- (Variables|Default|GetTime%20to%20Spawn%20Potato) DeltaSeconds)))))

(fn ConstructionScript)