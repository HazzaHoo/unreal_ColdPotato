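; Cold Potato pickup actor for a hot-potato style game, passed between the player and Hoarder, Opportunist and Interceptor AI.
; Separate floor-pickup and take spheres trigger handoffs that attach it to the holder's socket, slow them and update the timer widget.
; Losing it knocks back the previous holder, while dropping launches it behind them with physics.
; A cooldown and DoOnce gates limit repeat transfers, and saved difficulty sets the take radius.
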(event OnComponentBeginOverlap(FloorPickup_CollisionSphere)
  (params (OverlappedComponent :type Primitive%20Component%20Object%20Reference) (OtherActor :type Actor%20Object%20Reference) (OtherComp :type Primitive%20Component%20Object%20Reference) (OtherBodyIndex :type Integer) (bFromSweep :type Boolean) (SweepResult :type Hit%20Result%20Structure%20%28by%20ref%29))
  ;[0.15 0.15 0.15 0.5] Pickup (Start Game)
  (if (Variables|DropPotato|GetPotatoOnFloor?)
    (CallFunction|IdentifyPlayerCollided OtherActor)
    (CallFunction|PickupCooldown)))

(event OnComponentBeginOverlap(TakePotato_CollisionSphere)
  (params (OverlappedComponent :type Primitive%20Component%20Object%20Reference) (OtherActor :type Actor%20Object%20Reference) (OtherComp :type Primitive%20Component%20Object%20Reference) (OtherBodyIndex :type Integer) (bFromSweep :type Boolean) (SweepResult :type Hit%20Result%20Structure%20%28by%20ref%29))
  ;[0.15 0.15 0.15 0.5] Potato Collision
  (Variables|Default|SetOtherActorCollided OtherActor)
  (Utilities|FlowControl|DoOnce false
    (:Completed
      (Utilities|IsValid (Variables|Default|GetOtherActorCollided)
        (:Is%20Valid
          (if (Math|Boolean|ORBoolean (Variables|Cooldown|GetPickupCooldown) (Variables|DropPotato|GetPotatoOnFloor?) (== (Variables|ActorRefs|GetCharacterHoldingPotato) (Variables|Default|GetOtherActorCollided)) (Actor|ActorHasTag (Variables|Default|GetOtherActorCollided) "HeatLamp") (Actor|ActorHasTag (Variables|Default|GetOtherActorCollided) "Invis"))
            (CallFunction|ResetCollision :!label _label)
            (else
              (CallFunction|DetachPotatofromPlayer)
              (CallFunction|IdentifyPlayerCollided (Variables|Default|GetOtherActorCollided))
              (CallFunction|PickupCooldown))))
        (:Is%20Not%20Valid
          (goto _label))))))

(event Custom|Pickup%20Cooldown
  ;[0.15 0.15 0.15 0.5] Pickup Cooldown
  (Variables|Cooldown|SetPickupCooldown true)
  (Utilities|FlowControl|Delay (Variables|Cooldown|GetPickupCooldownTime))
  (Variables|Cooldown|SetPickupCooldown false)
  (CallFunction|ResetDropPotato)
  (CallFunction|ResetCollision))

(event Custom|DynamcMaterials
  ;[0.15 0.15 0.15 0.5] Set Dynamic Material
  (bind _returnvalue (Rendering|Material|CreateDynamicMaterialInstance "/Game/06_Assets/Potato/Textures/restaurant.restaurant" "None" "None" :!class /Script/Engine.KismetMaterialLibrary))
  (bind _output_get (Variables|Default|SetDynamicMaterial _returnvalue))
  (Rendering|Material|SetMaterial (Variables|Default|GetSM_Potato) 0 _output_get))

(event Custom|ForceOutOfPlayerHand
  (params (Other%20Actor :type Actor%20Object%20Reference))
  ;[0.15 0.15 0.15 0.5] Potato Collision
  (Variables|Default|SetOtherActorCollided Other%20Actor)
  (Utilities|FlowControl|DoOnce false
    (:Completed
      (Utilities|IsValid (Variables|Default|GetOtherActorCollided)
        (:Is%20Valid
          (if (Math|Boolean|ORBoolean (Variables|Cooldown|GetPickupCooldown) (Variables|DropPotato|GetPotatoOnFloor?) (== (Variables|ActorRefs|GetCharacterHoldingPotato) (Variables|Default|GetOtherActorCollided)) (Actor|ActorHasTag (Variables|Default|GetOtherActorCollided) "HeatLamp") (Actor|ActorHasTag (Variables|Default|GetOtherActorCollided) "Invis"))
            (CallFunction|ResetCollision :!label _label)
            (else
              (CallFunction|DetachPotatofromPlayer)
              (CallFunction|IdentifyPlayerCollided (Variables|Default|GetOtherActorCollided))
              (CallFunction|PickupCooldown))))
        (:Is%20Not%20Valid
          (goto _label))))))

(event Custom|Drop%20Potato
  ;[0.15 0.15 0.15 0.5] Drop Potato (Launch Behind Player Carrying it)
  (Utilities|FlowControl|DoOnce false
    (:Completed
      (CallFunction|DetachPotatofromPlayer)
      (CallFunction|DropPotato(Physics))
      (Variables|DropPotato|SetPotatoOnFloor? true))))

(event Custom|ResetDropPotato
  ;[0.15 0.15 0.15 0.5] Drop Potato (Launch Behind Player Carrying it)
  (Utilities|FlowControl|DoOnce false) ; enters at Reset
)

(event Custom|Reset%20Collision
  (bind _otheractorcollided (Variables|Default|GetOtherActorCollided))
  ;[0.15 0.15 0.15 0.5] Potato Collision
  (Utilities|FlowControl|DoOnce false) ; enters at Reset
)

(event EventBeginPlay
  ;[0.15 0.15 0.15 0.5] Get Timer Reference
  (bind _foundwidgets (Widget|GetAllWidgetsOfClass "/Game/05_UserInterface/Gameplay/WB_Timer.WB_Timer_C" true))
  (Variables|Widgets|SetTimerWB%20Ref (Utilities|Array|Get(acopy) _foundwidgets))
  (bind _asbp_first_person_character (Utilities|Casting|CastToBP_FirstPersonCharacter (Game|GetPlayerCharacter 0)))
  (Variables|ActorRefs|SetPlayer%20Ref _asbp_first_person_character)
  (CallFunction|DynamcMaterials)
  (CallFunction|SetDifficultyPickupSize)
  (bind _returnvalue (UserInterface|CreateWidget "/Game/05_UserInterface/Gameplay/WB_PotatoIcon.WB_PotatoIcon_C"))
  (UserInterface|Viewport|AddtoViewport _returnvalue 0))

(event EventTick
  (params (DeltaSeconds :type Float%20%28single-precision%29))
  ;[0.15 0.15 0.15 0.5] Rotate Icon to Player
  (CallFunction|RotateIcontoPlayer))

(fn ConstructionScript)

(fn IdentifyPlayerCollided
  (params (ActorCollided :type Actor%20Object%20Reference))
  (bind _asbp_first_person_character (Utilities|Casting|CastToBP_FirstPersonCharacter ActorCollided)
    (:then
      (Default|GotPotatoSpeedDecline _asbp_first_person_character)
      (Variables|/Game/01_PlayerCharacter/BP_FirstPersonCharacter.BP_FirstPersonCharacter_C|SetGotPotato? _asbp_first_person_character true)
      (Variables|ActorRefs|SetCharacterHoldingPotato _asbp_first_person_character)
      (CallFunction|AttachPotatotoPlayerCollided)
      (bind _returnvalue (UserInterface|CreateWidget "/Game/05_UserInterface/Gameplay/WB_GotLostPotato.WB_GotLostPotato_C"))
      (Default|SetText _returnvalue true)
      (UserInterface|Viewport|AddtoViewport _returnvalue 0))
    (:CastFailed
      (bind _asbp_ai_hoarder (Utilities|Casting|CastToBP_AI_Hoarder ActorCollided)
        (:then
          (bind _asai_hoarder_controller (Utilities|Casting|CastToAI_Hoarder_Controller (AI|GetAIController _asbp_ai_hoarder)))
          (Default|GotPotato _asai_hoarder_controller)
          (Variables|ActorRefs|SetCharacterHoldingPotato _asbp_ai_hoarder)
          (Default|GotPotatoSpeedDecline (Variables|/Game/03_AI-Enemies/AI_Parent_ControllerClass.AI_Parent_ControllerClass_C|GetController%20Pawn _asai_hoarder_controller)))
        (:CastFailed
          (bind _asbp_ai_oppertunist (Utilities|Casting|CastToBP_AI_Opportunist ActorCollided)
            (:then
              (bind _asai_oppertunist_controller (Utilities|Casting|CastToAI_Opportunist_Controller (AI|GetAIController _asbp_ai_oppertunist)))
              (Default|GotPotato _asai_oppertunist_controller)
              (Variables|ActorRefs|SetCharacterHoldingPotato _asbp_ai_oppertunist)
              (Default|GotPotatoSpeedDecline (Variables|/Game/03_AI-Enemies/AI_Parent_ControllerClass.AI_Parent_ControllerClass_C|GetController%20Pawn _asai_oppertunist_controller)))
            (:CastFailed
              (bind _asbp_ai_interceptor (Utilities|Casting|CastToBP_AI_Interceptor ActorCollided))
              (bind _asai_interceptor_controller (Utilities|Casting|CastToAI_Interceptor_Controller (AI|GetAIController _asbp_ai_interceptor)))
              (Default|GotPotato _asai_interceptor_controller)
              (Variables|ActorRefs|SetCharacterHoldingPotato _asbp_ai_interceptor)
              (Default|GotPotatoSpeedDecline (Variables|/Game/03_AI-Enemies/AI_Parent_ControllerClass.AI_Parent_ControllerClass_C|GetController%20Pawn _asai_interceptor_controller))))))
      (CallFunction|AttachPotatotoPlayerCollided))))

(fn AttachPotatotoPlayerCollided
  (Physics|SetSimulatePhysics (Variables|Default|GetSM_Potato) false)
  (Variables|Default|SetPotatoParentMesh (Variables|/Script/Engine.Character|GetMesh (Variables|ActorRefs|GetCharacterHoldingPotato)))
  (if (Variables|DropPotato|GetPotatoOnFloor?)
    ;[0.15 0.15 0.15 0.5] Disable Floor Collision
    (Collision|SetCollisionEnabled (Variables|Default|GetFloorPickup_CollisionSphere) "NoCollision")
    (Collision|SetCollisionEnabled (Variables|Default|GetTakePotato_CollisionSphere) "QueryAndPhysics")
    (Variables|DropPotato|SetPotatoOnFloor? false))
  (Transformation|AttachComponentToComponent (Variables|Default|GetPotatoParentMesh) "POTATO" "SnapToTarget" "KeepRelative" "KeepWorld" true)
  (Default|WhoHasPotato (Variables|Widgets|GetTimerWB%20Ref) (Variables|ActorRefs|GetCharacterHoldingPotato))
  ;[0.15 0.15 0.15 0.5] Make Potato Correct Size
  (Transformation|SetRelativeScale3D (Variables|Default|GetSM_Potato) "0.370000,0.370000,0.370000"))

(fn DetachPotatofromPlayer
  (bind _characterholdingpotato (Variables|ActorRefs|GetCharacterHoldingPotato))
  (bind _asbp_first_person_character (Utilities|Casting|CastToBP_FirstPersonCharacter _characterholdingpotato)
    (:then
      (Variables|/Game/01_PlayerCharacter/BP_FirstPersonCharacter.BP_FirstPersonCharacter_C|SetGotPotato? _asbp_first_person_character false)
      (bind _returnvalue (UserInterface|CreateWidget "/Game/05_UserInterface/Gameplay/WB_GotLostPotato.WB_GotLostPotato_C"))
      (Default|SetText _returnvalue false)
      (UserInterface|Viewport|AddtoViewport _returnvalue 0)
      (CallFunction|LostPotatoKnockback 0 true))
    (:CastFailed
      (bind _asbp_ai_hoarder (Utilities|Casting|CastToBP_AI_Hoarder _characterholdingpotato)
        (:then
          (bind _asai_hoarder_controller (Utilities|Casting|CastToAI_Hoarder_Controller (AI|GetAIController _asbp_ai_hoarder)))
          (Default|LostPotato _asai_hoarder_controller)
          (CallFunction|LostPotatoKnockback _asbp_ai_hoarder false _asai_hoarder_controller)
          (Variables|/Game/03_AI-Enemies/BP_AI_ParentClass.BP_AI_ParentClass_C|SetGotPotato? _asbp_ai_hoarder false))
        (:CastFailed
          (bind _asbp_ai_oppertunist (Utilities|Casting|CastToBP_AI_Opportunist _characterholdingpotato)
            (:then
              (bind _asai_oppertunist_controller (Utilities|Casting|CastToAI_Opportunist_Controller (AI|GetAIController _asbp_ai_oppertunist)))
              (Default|LostPotato _asai_oppertunist_controller)
              (CallFunction|LostPotatoKnockback _asbp_ai_oppertunist false _asai_oppertunist_controller)
              (Variables|/Game/03_AI-Enemies/BP_AI_ParentClass.BP_AI_ParentClass_C|SetGotPotato? _asbp_ai_oppertunist false))
            (:CastFailed
              (bind _asbp_ai_interceptor (Utilities|Casting|CastToBP_AI_Interceptor _characterholdingpotato))
              (bind _asai_interceptor_controller (Utilities|Casting|CastToAI_Interceptor_Controller (AI|GetAIController _asbp_ai_interceptor)))
              (Default|LostPotato _asai_interceptor_controller)
              (CallFunction|LostPotatoKnockback _asbp_ai_interceptor false _asai_interceptor_controller)
              (Variables|/Game/03_AI-Enemies/BP_AI_ParentClass.BP_AI_ParentClass_C|SetGotPotato? _asbp_ai_interceptor false))))))))

(fn DropPotato(Physics)
  (bind _sm_potato (Variables|Default|GetSM_Potato))
  (Utilities|IsValid (Variables|ActorRefs|GetCharacterHoldingPotato)
    (:Is%20Valid
      (Collision|SetCollisionEnabled (Variables|Default|GetTakePotato_CollisionSphere) "NoCollision")
      (Collision|SetCollisionEnabled (Variables|Default|GetFloorPickup_CollisionSphere) "QueryAndPhysics")
      ;[0.15 0.15 0.15 0.5] This makes Potato Shrink
      (Physics|SetSimulatePhysics _sm_potato true)
      (Class|PrimitiveComponent|WakeRigidBody _sm_potato "None")
      ;[0.15 0.15 0.15 0.5] Make Potato Right Size
      (Transformation|SetRelativeScale3D _sm_potato "0.370000,0.370000,0.370000")
      (Physics|AddImpulse _sm_potato (Math|Vector|MakeVector (* (* (.X (Math|Vector|BreakVector (Transformation|GetActorForwardVector (Variables|ActorRefs|GetCharacterHoldingPotato)))) -1.0) (Variables|DropPotato|GetX%20Potato%20Lauch%20Multiplier)) 0.0 (Variables|DropPotato|GetZ%20Potato%20Launch%20Multiplier)) "None" true)
      (Default|WhoHasPotato (Variables|Widgets|GetTimerWB%20Ref)))))

(fn RotateIcontoPlayer)

(fn SetDifficultyPickupSize
  (bind _takepotato_collisionsphere (Variables|Default|GetTakePotato_CollisionSphere))
  (bind _returnvalue (Actor|GetActorOfClass "/Game/04_Blueprints/Manager/BP_Manager.BP_Manager_C"))
  (switch int (Variables|/Game/04_Blueprints/BP_PotatoSaveGame.BP_PotatoSaveGame_C|GetDifficultySetting (Variables|/Game/04_Blueprints/Manager/BP_Manager.BP_Manager_C|GetSave%20Game%20Ref _returnvalue))
    (:0
      (Transformation|SetRelativeScale3D _takepotato_collisionsphere (Variables|Difficulty|GetEasyDifficultySize)))
    (:1
      (Transformation|SetRelativeScale3D _takepotato_collisionsphere (Variables|Difficulty|GetMediumDifficultySize)))
    (:2
      (Transformation|SetRelativeScale3D _takepotato_collisionsphere (Variables|Difficulty|GetHardDifficultySize)))))

(fn GameEnded
  (Collision|SetCollisionEnabled (Variables|Default|GetTakePotato_CollisionSphere) "NoCollision"))

(fn LostPotatoKnockback
  (params (LostPotatoActor :type BP%20AI%20Parent%20Class%20Object%20Reference) (KnockbackPlayer? :type Boolean) (Lost%20Potato%20Actor%20Controller :type AI%20Parent%20Controller%20Class%20Object%20Reference))
  (if KnockbackPlayer?
    (bind _asbp_first_person_character (Utilities|Casting|CastToBP_FirstPersonCharacter (Game|GetPlayerCharacter 0)))
    (Default|LaunchCharacter _asbp_first_person_character)
    (Default|ResetWalkSpeed _asbp_first_person_character)
    (else
      (Utilities|IsValid LostPotatoActor
        (:Is%20Valid
          (Default|LaunchPlayer LostPotatoActor Lost%20Potato%20Actor%20Controller)
          (Default|ResetWalkSpeed LostPotatoActor))))))