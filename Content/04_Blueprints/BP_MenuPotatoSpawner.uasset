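; Menu potato spawner actor that endlessly drops physics-simulated, shadowless potato mesh components at a spawn point.
; BeginPlay starts a self-repeating loop that adds each potato to an array, then waits a short random delay.
; Once the count reaches the cap, each cycle removes the first array entry, then destroys the component now at index zero.
; SpawnMorePotatoes runs the same spawn step in a horde-sized loop while under the cap.
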(event Custom|LoopPotatoSpawn
  (bind _potatoarray (Variables|Default|GetPotatoArray))
  (bind _output (Utilities|Array|Get(acopy) _potatoarray))
  (if (>= (Variables|Default|GetAmountOfPotatos) (Variables|Default|GetMaxAmountOfPotatos))
    (Utilities|Array|RemoveItem _potatoarray _output)
    (Components|DestroyComponent _output))
  (bind _returnvalue (AddComponent|AddStaticMeshComponent true (Transformation|GetWorldTransform (Variables|Default|GetPotato_SpawnPoint))))
  (bind _returnvalue_2 (Utilities|Array|Add (Variables|Default|GetPotatoArray) _returnvalue))
  (Development|PrintString (Utilities|String|ToString(Integer) _returnvalue_2))
  (Components|StaticMesh|SetStaticMesh _returnvalue "/Game/06_Assets/Potato/SM_Potato.SM_Potato")
  (Rendering|SetCastShadow _returnvalue false)
  (Physics|SetSimulatePhysics _returnvalue true)
  (Utilities|FlowControl|Delay (Math|Random|RandomFloatinRange 0.1 0.5))
  (Math|Integer|IncrementInt (Variables|Default|GetAmountOfPotatos)
    (:%20%20
      (CallFunction|LoopPotatoSpawn))))

(event Custom|SpawnMorePotatoes
  (if (not (>= (Variables|Default|GetAmountOfPotatos) (Variables|Default|GetMaxAmountOfPotatos)))
    (for _index (range 0 (Variables|Default|GetPotatoHordeAmt))
      (bind _returnvalue (AddComponent|AddStaticMeshComponent true (Transformation|GetWorldTransform (Variables|Default|GetPotato_SpawnPoint))))
      (bind _returnvalue_2 (Utilities|Array|Add (Variables|Default|GetPotatoArray) _returnvalue))
      (Development|PrintString (Utilities|String|ToString(Integer) _returnvalue_2))
      (Components|StaticMesh|SetStaticMesh _returnvalue "/Game/06_Assets/Potato/SM_Potato.SM_Potato")
      (Rendering|SetCastShadow _returnvalue false)
      (Physics|SetSimulatePhysics _returnvalue true)
      (Utilities|FlowControl|Delay (Math|Random|RandomFloatinRange 0.1 0.5))
      (Math|Integer|IncrementInt (Variables|Default|GetAmountOfPotatos)
        (:%20%20
          (CallFunction|LoopPotatoSpawn))))))

(event EventBeginPlay
  (bind _returnvalue (AddComponent|AddStaticMeshComponent true (Transformation|GetWorldTransform (Variables|Default|GetPotato_SpawnPoint))))
  (bind _returnvalue_2 (Utilities|Array|Add (Variables|Default|GetPotatoArray) _returnvalue))
  (Development|PrintString (Utilities|String|ToString(Integer) _returnvalue_2))
  (Components|StaticMesh|SetStaticMesh _returnvalue "/Game/06_Assets/Potato/SM_Potato.SM_Potato")
  (Rendering|SetCastShadow _returnvalue false)
  (Physics|SetSimulatePhysics _returnvalue true)
  (Utilities|FlowControl|Delay (Math|Random|RandomFloatinRange 0.1 0.5))
  (Math|Integer|IncrementInt (Variables|Default|GetAmountOfPotatos)
    (:%20%20
      (CallFunction|LoopPotatoSpawn))))

(fn ConstructionScript)