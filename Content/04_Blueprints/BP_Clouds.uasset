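; Cloud ring actor that surrounds its centre with randomly chosen cloud meshes and rotates them as a backdrop.
; On BeginPlay, once the player casts to BP_FirstPersonCharacter, SpawnClouds adds mesh components at even angular steps with random radius and height.
; Each cloud is turned toward the centre with an added pitch offset.
; The CircleMap timeline then rotates the whole actor through a lerped full turn, carrying the clouds around.
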(event EventBeginPlay
  ;[0.15 0.15 0.15 0.5] Rotate around centre
  (bind _asbp_first_person_character (Utilities|Casting|CastToBP_FirstPersonCharacter (Game|GetPlayerCharacter 0)))
  (Variables|Default|SetPlayer%20Ref _asbp_first_person_character)
  (CallFunction|SpawnClouds)
  (bind _lerp (Timeline|CircleMap Play)
    (:Update
      (Transformation|SetActorRotation (Math|Rotator|Lerp(Rotator) "0, 0, 0" "0.000000,360.000000,0.000000" _lerp)))))

(fn ConstructionScript)

(fn SpawnClouds
  (bind _defaultsceneroot (Variables|Default|GetDefaultSceneRoot))
  (bind _amount_of_clouds (Variables|Default|GetAmount%20of%20Clouds))
  (bind _relativelocation (Variables|/Script/Engine.SceneComponent|GetRelativeLocation _defaultsceneroot))
  (for _index (range 1 _amount_of_clouds)
    (bind _returnvalue (AddComponent|AddStaticMeshComponent false))
    (Variables|Default|SetCloudMeshReference _returnvalue)
    (switch int (Math|Random|RandomIntegerinRange 0 2)
      (:0
        (Components|StaticMesh|SetStaticMesh (Variables|Default|GetCloudMeshReference) "/Game/06_Assets/AssetPacks/Cloud_Models/Cloud_03.Cloud_03"))
      (:1
        (Components|StaticMesh|SetStaticMesh (Variables|Default|GetCloudMeshReference) "/Game/06_Assets/AssetPacks/Cloud_Models/Cloud_01.Cloud_01"))
      (:2
        (Components|StaticMesh|SetStaticMesh (Variables|Default|GetCloudMeshReference) "/Game/06_Assets/AssetPacks/Cloud_Models/Cloud_02.Cloud_02")))
    (Transformation|SetRelativeRotation (Variables|Default|GetCloudMeshReference) (Math|Rotator|MakeRotator (.roll (Math|Rotator|FindLookatRotation (+ (* (Math|Vector|GetForwardVector (Math|Rotator|MakeRotator 0.0 0.0 (Math|Conversions|ToFloat(Integer) (* _index (/ 360 _amount_of_clouds))))) (* (Math|Random|RandomFloatinRange (Variables|Default|GetMinRadius) (Variables|Default|GetMaxRadius)) 1e+02)) _relativelocation) (Transformation|GetWorldLocation (Variables|Default|GetDefaultSceneRoot)))) (+ (.pitch (Math|Rotator|FindLookatRotation (+ (* (Math|Vector|GetForwardVector (Math|Rotator|MakeRotator 0.0 0.0 (Math|Conversions|ToFloat(Integer) (* _index (/ 360 _amount_of_clouds))))) (* (Math|Random|RandomFloatinRange (Variables|Default|GetMinRadius) (Variables|Default|GetMaxRadius)) 1e+02)) _relativelocation) (Transformation|GetWorldLocation (Variables|Default|GetDefaultSceneRoot)))) (Variables|Default|GetCloud%20Pitch)) (.yaw (Math|Rotator|FindLookatRotation (+ (* (Math|Vector|GetForwardVector (Math|Rotator|MakeRotator 0.0 0.0 (Math|Conversions|ToFloat(Integer) (* _index (/ 360 _amount_of_clouds))))) (* (Math|Random|RandomFloatinRange (Variables|Default|GetMinRadius) (Variables|Default|GetMaxRadius)) 1e+02)) _relativelocation) (Transformation|GetWorldLocation (Variables|Default|GetDefaultSceneRoot))))) false false)
    (Transformation|SetWorldLocation (Variables|Default|GetCloudMeshReference) (Math|Vector|MakeVector (.X (Math|Vector|BreakVector (+ (* (Math|Vector|GetForwardVector (Math|Rotator|MakeRotator 0.0 0.0 (Math|Conversions|ToFloat(Integer) (* _index (/ 360 _amount_of_clouds))))) (* (Math|Random|RandomFloatinRange (Variables|Default|GetMinRadius) (Variables|Default|GetMaxRadius)) 1e+02)) _relativelocation))) (.Y (Math|Vector|BreakVector (+ (* (Math|Vector|GetForwardVector (Math|Rotator|MakeRotator 0.0 0.0 (Math|Conversions|ToFloat(Integer) (* _index (/ 360 _amount_of_clouds))))) (* (Math|Random|RandomFloatinRange (Variables|Default|GetMinRadius) (Variables|Default|GetMaxRadius)) 1e+02)) _relativelocation))) (+ (.Z (Math|Vector|BreakVector _relativelocation)) (Math|Random|RandomFloatinRange -2e+02 5e+02))) false false)))