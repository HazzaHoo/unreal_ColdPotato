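; Debug telemetry actor that records a movement heat map of the player and AI types across the level.
; On BeginPlay it spawns a grid of cube meshes with dynamic materials, whose overlaps raise total and per-character-type scalar parameters.
; Backspace toggles the cubes, legend widget and camera view.
; Number keys switch the heat map filter or, in debug mode, hide the heat lamp, characters and potato.
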(event Custom|Loop%20Box%20Collision%20Spawn
  ;[0.15 0.15 0.15 0.5] Spawn Box In Row
  (Utilities|FlowControl|Delay 0.001)
  (if (== (Variables|SpawnBoxes|GetWidth) 0)
    (CallFunction|ShiftRowDown)
    (CallFunction|LoopBoxCollisionSpawn)
    (else
      (CallFunction|ShiftRowLeft&AssignMaterial (delegate Custom|OnComponentBeginOverlap_Event))
      (CallFunction|LoopBoxCollisionSpawn))))

(event Custom|OnComponentBeginOverlap_Event
  (params (OverlappedComponent :type Primitive%20Component%20Object%20Reference) (OtherActor :type Actor%20Object%20Reference) (OtherComp :type Primitive%20Component%20Object%20Reference) (OtherBodyIndex :type Integer) (bFromSweep :type Boolean) (SweepResult :type Hit%20Result%20Structure%20%28by%20ref%29))
  ;[0.15 0.15 0.15 0.5] Up[date Cube Colour (On Event)
  (if (not (Actor|ActorHasTag OtherActor "HeatLamp"))
    (CallFunction|UpdateBoxColours (.hitcomponent SweepResult) OtherActor)))

(event Custom|Set%20Heat%20Map%20Player%20View
  (params (ViewNum :type Float%20%28double-precision%29))
  ;[0.15 0.15 0.15 0.5] 1-5 Nums to select Heat Map Mode
  ;;[0.15 0.15 0.15 0.5] Set Player Scalar Switch
  (for _array_element (Variables|Default|GetCubeMIDs)
    (Rendering|Material|SetScalarParameterValue _array_element "ViewSwitch(1-5)" ViewNum :!class /Script/Engine.MaterialInstanceDynamic)))

(event Custom|Set%20Player%20Scalar%20Parameters
  (params (Parameter%20Name :type Name) (Dynamic%20Material :type Material%20Instance%20Dynamic%20Object%20Reference))
  ;[0.15 0.15 0.15 0.5] 1-5 Nums to select Heat Map Mode
  ;;[0.15 0.15 0.15 0.5] Set Player Scalar Switch
  (bind _returnvalue (Rendering|Material|GetScalarParameterValue Dynamic%20Material Parameter%20Name :!class /Script/Engine.MaterialInstanceDynamic))
  (Rendering|Material|SetScalarParameterValue Dynamic%20Material Parameter%20Name (+ _returnvalue 0.1) :!class /Script/Engine.MaterialInstanceDynamic))

(event Custom|SpawnDebugWidget
  ;[0.15 0.15 0.15 0.5] Spawn Debug Widget
  (bind _returnvalue (UserInterface|CreateWidget "/Game/05_UserInterface/WB_DebugLegend.WB_DebugLegend_C"))
  (bind _output_get (Variables|Default|SetDebugWidget _returnvalue))
  (UserInterface|Viewport|AddtoViewport _returnvalue 0)
  (Widget|SetVisibility _output_get "Hidden"))

(event EventBeginPlay
  (bind _width (Variables|SpawnBoxes|GetWidth))
  ;[0.15 0.15 0.15 0.5] Spawn Box In Row
  (CallFunction|SpawnDebugWidget)
  (bind _asbp_first_person_character (Utilities|Casting|CastToBP_FirstPersonCharacter (Game|GetPlayerCharacter 0)))
  (Variables|Default|SetPlayer%20REF _asbp_first_person_character)
  (Input|EnableInput (Game|GetPlayerController 0))
  (if (Variables|Debug|GetTurnOn)
    (Variables|SpawnBoxes|SetResetWidthVar _width)
    (if (== _width 0)
      (CallFunction|ShiftRowDown)
      (CallFunction|LoopBoxCollisionSpawn)
      (else
        (CallFunction|ShiftRowLeft&AssignMaterial (delegate Custom|OnComponentBeginOverlap_Event))
        (CallFunction|LoopBoxCollisionSpawn)))))

(event Input|KeyboardEvents|Backspace
  (params (Key :type Key%20Structure :default "None"))
  ;[0.15 0.15 0.15 0.5] 1-5 Nums to select Heat Map Mode
  ;;[0.15 0.15 0.15 0.5] Hide or Show Telemetry
  (:Pressed
    (CallFunction|HideorShowTelemetry)))

(event Input|KeyboardEvents|1
  (params (Key :type Key%20Structure :default "None"))
  ;[0.15 0.15 0.15 0.5] 1-5 Nums to select Heat Map Mode
  ;;[0.15 0.15 0.15 0.5] Heat Map Filter
  (:Pressed
    (CallFunction|SetHeatMapPlayerView 0.0)))

(event Input|KeyboardEvents|2
  (params (Key :type Key%20Structure :default "None"))
  ;[0.15 0.15 0.15 0.5] 1-5 Nums to select Heat Map Mode
  ;;[0.15 0.15 0.15 0.5] Heat Map Filter
  (:Pressed
    (CallFunction|SetHeatMapPlayerView 1.0)))

(event Input|KeyboardEvents|3
  (params (Key :type Key%20Structure :default "None"))
  ;[0.15 0.15 0.15 0.5] 1-5 Nums to select Heat Map Mode
  ;;[0.15 0.15 0.15 0.5] Heat Map Filter
  (:Pressed
    (CallFunction|SetHeatMapPlayerView 2.0)))

(event Input|KeyboardEvents|4
  (params (Key :type Key%20Structure :default "None"))
  ;[0.15 0.15 0.15 0.5] 1-5 Nums to select Heat Map Mode
  ;;[0.15 0.15 0.15 0.5] Heat Map Filter
  (:Pressed
    (CallFunction|SetHeatMapPlayerView 3.0)))

(event Input|KeyboardEvents|5
  (params (Key :type Key%20Structure :default "None"))
  ;[0.15 0.15 0.15 0.5] 1-5 Nums to select Heat Map Mode
  ;;[0.15 0.15 0.15 0.5] Heat Map Filter
  (:Pressed
    (CallFunction|SetHeatMapPlayerView 4.0)))

(event Input|KeyboardEvents|6
  (params (Key :type Key%20Structure :default "None"))
  ;[0.15 0.15 0.15 0.5] 1-5 Nums to select Heat Map Mode
  ;;[0.15 0.15 0.15 0.5] Hide or Show Heat Lamp
  (:Pressed
    (if (Variables|Debug|GetDebugMode?)
      (bind _outactors (Actor|GetAllActorsOfClass "/Game/04_Blueprints/HeatLamp/BP_HeatLamp.BP_HeatLamp_C"))
      (if (Rendering|IsVisible (Variables|/Script/Engine.Actor|GetRootComponent (Utilities|Array|Get(acopy) _outactors)))
        (Rendering|SetVisibility (Variables|/Script/Engine.Actor|GetRootComponent (Utilities|Array|Get(acopy) _outactors)) false true)
        (else
          (Rendering|SetVisibility (Variables|/Script/Engine.Actor|GetRootComponent (Utilities|Array|Get(acopy) _outactors)) true true))))))

(event Input|KeyboardEvents|7
  (params (Key :type Key%20Structure :default "None"))
  ;[0.15 0.15 0.15 0.5] 1-5 Nums to select Heat Map Mode
  ;;[0.15 0.15 0.15 0.5] Hide Players & Potato
  (:Pressed
    (if (Variables|Debug|GetDebugMode?)
      (bind _outactors (Actor|GetAllActorsOfClass "/Game/04_Blueprints/ColdPotato_BP.ColdPotato_BP_C"))
      (Utilities|IsValid (Utilities|Array|Get(acopy) _outactors)
        (:Is%20Valid
          (if (Variables|/Script/Engine.Actor|GetbHidden (Utilities|Array|Get(acopy) _outactors))
            (Rendering|SetActorHiddenInGame (Utilities|Array|Get(acopy) _outactors) false)
            (else
              (Rendering|SetActorHiddenInGame (Utilities|Array|Get(acopy) _outactors) true))))
        (:Is%20Not%20Valid
          _))
      (bind _outactors_2 (Actor|GetAllActorsOfClass "/Game/04_Blueprints/BP_Manager.BP_Manager_C"))
      (for _array_element (Variables|/Game/04_Blueprints/BP_Manager.BP_Manager_C|GetPlayers (Utilities|Array|Get(acopy) _outactors_2))
        (if (Variables|/Script/Engine.Actor|GetbHidden _array_element)
          (Rendering|SetActorHiddenInGame _array_element false)
          (else
            (Rendering|SetActorHiddenInGame _array_element true)))))))

(fn ConstructionScript)

(fn ShiftRowDown
  (Variables|SpawnBoxes|SetWidth (Variables|SpawnBoxes|GetResetWidthVar))
  (if (not (== (Variables|SpawnBoxes|GetLength) 0))
    (Math|Integer|DecrementInt (Variables|SpawnBoxes|GetLength)
      (:%20%20
        (Variables|SpawnBoxes|SetSpawnBoxTransform (Math|Transform|MakeTransform (Math|Vector|MakeVector 0.0 (+ (.Y (Math|Vector|BreakVector (.location (Variables|SpawnBoxes|GetSpawnBoxTransform)))) 1.9e+02) 0.0) (.rotation (Variables|SpawnBoxes|GetSpawnBoxTransform)) (.scale (Variables|SpawnBoxes|GetSpawnBoxTransform))))))))

(fn ShiftRowLeft&AssignMaterial
  (params (Event%20on%20Overlap%20Event :type Delegate%20%28by%20ref%29))
  (bind _returnvalue (AddComponent|AddStaticMeshComponent false (Math|Transform|MakeTransform (.Location (Math|Transform|BreakTransform (Variables|SpawnBoxes|GetSpawnBoxTransform))) (.Rotation (Math|Transform|BreakTransform (Variables|SpawnBoxes|GetSpawnBoxTransform))) (.Scale (Math|Transform|BreakTransform (Variables|SpawnBoxes|GetSpawnBoxTransform))))))
  (Utilities|Array|Add (Variables|Default|GetCubeMeshes) _returnvalue)
  (Collision|SetCollisionProfileName _returnvalue "Telementry" false :!class /Script/Engine.PrimitiveComponent)
  (Components|StaticMesh|SetStaticMesh _returnvalue "/Game/00_LevelPrototyping/Meshes/SM_ChamferCube.SM_ChamferCube")
  (bind _returnvalue_2 (Rendering|Material|CreateDynamicMaterialInstance "/Game/04_Blueprints/M_Telementry.M_Telementry" "None" "None" :!class /Script/Engine.KismetMaterialLibrary))
  (Rendering|Material|SetMaterial _returnvalue 0 _returnvalue_2)
  (Utilities|Array|Add (Variables|Default|GetCubeMIDs) _returnvalue_2)
  (Collision|BindEventtoOnComponentBeginOverlap _returnvalue Event%20on%20Overlap%20Event)
  (Development|SetHiddeninGame _returnvalue (Variables|Debug|GetHideTelementryBoxes) false)
  (Math|Integer|DecrementInt (Variables|SpawnBoxes|GetWidth)
    (:%20%20
      (Variables|SpawnBoxes|SetSpawnBoxTransform (Math|Transform|MakeTransform (Math|Vector|MakeVector (+ (.X (Math|Vector|BreakVector (Variables|/Script/Engine.SceneComponent|GetRelativeLocation _returnvalue))) (Variables|SpawnBoxes|GetWidthTranslation)) (.Y (Math|Vector|BreakVector (Variables|/Script/Engine.SceneComponent|GetRelativeLocation _returnvalue))) (.Z (Math|Vector|BreakVector (Variables|/Script/Engine.SceneComponent|GetRelativeLocation _returnvalue)))) "0, 0, 0" "2.000000,2.000000,2.000000")))))

(fn UpdateBoxColours
  (params (Hit%20Component :type Primitive%20Component%20Object%20Reference) (Other%20Actor :type Actor%20Object%20Reference))
  (for (_array_element _array_index) (Variables|Default|GetCubeMeshes)
    (if (== _array_element Hit%20Component)
      (bind _returnvalue (Rendering|Material|GetScalarParameterValue (Utilities|Array|Get(acopy) (Variables|Default|GetCubeMIDs) _array_index) "PassingByValues" :!class /Script/Engine.MaterialInstanceDynamic))
      (Rendering|Material|SetScalarParameterValue (Utilities|Array|Get(acopy) (Variables|Default|GetCubeMIDs) _array_index) "PassingByValues" (+ _returnvalue 0.1) :!class /Script/Engine.MaterialInstanceDynamic)
      (Utilities|Casting|CastToBP_FirstPersonCharacter Other%20Actor
        (:then
          (CallFunction|SetPlayerScalarParameters "PassingByValuesPLAYER" (Utilities|Array|Get(acopy) (Variables|Default|GetCubeMIDs) _array_index)))
        (:CastFailed
          (Utilities|Casting|CastToBP_AI_Hoarder Other%20Actor
            (:then
              (CallFunction|SetPlayerScalarParameters "PassingByValuesHOARDER" (Utilities|Array|Get(acopy) (Variables|Default|GetCubeMIDs) _array_index)))
            (:CastFailed
              (Utilities|Casting|CastToBP_AI_Interceptor Other%20Actor
                (:then
                  (CallFunction|SetPlayerScalarParameters "PassingByValuesINTERCEPTOR" (Utilities|Array|Get(acopy) (Variables|Default|GetCubeMIDs) _array_index)))
                (:CastFailed
                  (Utilities|Casting|CastToBP_AI_Oppertunist Other%20Actor)
                  (CallFunction|SetPlayerScalarParameters "PassingByValuesOPPERTUNIST" (Utilities|Array|Get(acopy) (Variables|Default|GetCubeMIDs) _array_index)))))))))))

(fn HideorShowTelemetry
  (bind _returnvalue (Game|GetPlayerController 0))
  (bind _debugwidget (Variables|Default|GetDebugWidget))
  (bind _cubemeshes (Variables|Default|GetCubeMeshes))
  (if (Variables|Debug|GetHideTelementryBoxes)
    (for _array_element _cubemeshes
      (Development|SetHiddeninGame _array_element false false)
      (Game|Player|SetViewTargetwithBlend _returnvalue self 0.0 "VTBlend_Linear" 0.0 false)
      (Widget|SetVisibility _debugwidget "Visible")
      (Variables|Debug|SetDebugMode? true))
    (Variables|Debug|SetHideTelementryBoxes false)
    (else
      (for _array_element_2 _cubemeshes
        (Development|SetHiddeninGame _array_element_2 true false)
        (Game|Player|SetViewTargetwithBlend _returnvalue (Variables|Default|GetPlayer%20REF) 0.0 "VTBlend_Linear" 0.0 false)
        (Widget|SetVisibility _debugwidget "Hidden")
        (Variables|Debug|SetDebugMode? false))
      (Variables|Debug|SetHideTelementryBoxes true))))