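; Parent character class for AI NPCs in a potato-passing game, with a player-facing name tag and configurable mesh material.
; Getting the potato starts a Timeline that lowers walk speed, while close-quarter overlaps with an NPC or player force the potato out of hand, throttled by a resetting DoOnce.
; Knockback launches the character away from the ColdPotato, flags its AI controller's blackboard key and briefly disables capsule overlap events.
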(event OnComponentBeginOverlap(CloseQuaterCollision)
  (params (OverlappedComponent :type Primitive%20Component%20Object%20Reference) (OtherActor :type Actor%20Object%20Reference) (OtherComp :type Primitive%20Component%20Object%20Reference) (OtherBodyIndex :type Integer) (bFromSweep :type Boolean) (SweepResult :type Hit%20Result%20Structure%20%28by%20ref%29))
  (if (and (or (Actor|ActorHasTag OtherActor "NPC") (Actor|ActorHasTag OtherActor "Player")) (Variables|Default|GetGotPotato?))
    (Utilities|FlowControl|DoOnce false :!label _label
      (:Completed
        (Default|ForceOutOfPlayerHand (Variables|Default|GetCold%20Potato%20Ref) OtherActor)
        (Utilities|FlowControl|Delay 1.0)
        (goto _label Reset)))))

(event Custom|GotPotatoSpeedDecline
  (bind _getmaxwalkspeed (Variables|Default|GetGetMaxWalkSpeed))
  (Variables|Default|SetGotPotato? true)
  (bind _lerp (Timeline|Timeline Play)
    (:Update
      (Variables|/Script/Engine.CharacterMovementComponent|SetMaxWalkSpeed (Variables|Character|GetCharacterMovement) (Math|Float|Lerp _getmaxwalkspeed (- _getmaxwalkspeed 1.5e+02) _lerp)))))

(event Custom|Knockback%20Disable%20Collision
  ;[0.15 0.15 0.15 0.5] Knockback Disable Collision
  (Variables|/Script/Engine.PrimitiveComponent|SetbGenerateOverlapEvents (Variables|Collision|GetCapsuleComponent) false)
  (Utilities|FlowControl|Delay (Variables|Default|GetKnockback%20Collision%20Time))
  (Variables|/Script/Engine.PrimitiveComponent|SetbGenerateOverlapEvents (Variables|Collision|GetCapsuleComponent) true))

(event Custom|Reset%20Walk%20Speed
  (bind _getmaxwalkspeed (Variables|Default|GetGetMaxWalkSpeed))
  (CallFunction|UpdateWalkSpeed (Variables|Default|GetGetMaxWalkSpeed))
  (bind _lerp (Timeline|Timeline Stop)
    (:Update
      (Variables|/Script/Engine.CharacterMovementComponent|SetMaxWalkSpeed (Variables|Character|GetCharacterMovement) (Math|Float|Lerp _getmaxwalkspeed (- _getmaxwalkspeed 1.5e+02) _lerp)))))

(event EventBeginPlay
  ;[0.15 0.15 0.15 0.5] Set Name tag and Material to Player Type
  (bind _asbp_first_person_character (Utilities|Casting|CastToBP_FirstPersonCharacter (Game|GetPlayerCharacter 0)))
  (Variables|Default|SetPlayer%20Ref _asbp_first_person_character)
  (Rendering|Components|TextRender|SetText (Variables|Default|GetTextRender) (Variables|Default|GetNameTag))
  (Rendering|Material|SetMaterial (Variables|Character|GetMesh) 0 (Variables|Default|GetCharacerMesh_Material)))

(event EventTick
  (params (DeltaSeconds :type Float%20%28single-precision%29))
  ;[0.15 0.15 0.15 0.5] Rotate Name to Player
  (CallFunction|RotateNametoPlayer))

(fn ConstructionScript)

(fn UpdateWalkSpeed
  (params (NewWalkSpeed :type Float%20%28double-precision%29))
  (bind _output_get (Variables|/Script/Engine.CharacterMovementComponent|SetMaxWalkSpeed (Variables|Character|GetCharacterMovement) NewWalkSpeed))
  (Variables|Default|SetGetMaxWalkSpeed _output_get))

(fn RotateNametoPlayer
  (Transformation|SetWorldRotation (Variables|Default|GetTextRender) (Math|Rotator|FindLookatRotation (Transformation|GetActorLocation) (Transformation|GetActorLocation (Variables|Default|GetPlayer%20Ref))) false false))

(fn LaunchPlayer
  (params (AI%20Controller :type AI%20Parent%20Controller%20Class%20Object%20Reference))
  (bind _returnvalue (Actor|GetActorOfClass "/Game/04_Blueprints/ColdPotato_BP.ColdPotato_BP_C"))
  (Default|KnockbackBBKey AI%20Controller)
  (Character|LaunchCharacter self (Math|Vector|MakeVector (.X (Math|Vector|BreakVector (* (Math|Vector|GetForwardVector (Math|Rotator|FindLookatRotation (Transformation|GetActorLocation _returnvalue) (Transformation|GetActorLocation))) (* (Variables|Default|GetLaunchCharacterMulti) 1e+01)))) (.Y (Math|Vector|BreakVector (* (Math|Vector|GetForwardVector (Math|Rotator|FindLookatRotation (Transformation|GetActorLocation _returnvalue) (Transformation|GetActorLocation))) (* (Variables|Default|GetLaunchCharacterMulti) 1e+01)))) 6e+02) true true)
  (CallFunction|KnockbackDisableCollision))

(fn GetPotatoRef
  (bind _returnvalue (Actor|GetActorOfClass "/Game/04_Blueprints/ColdPotato_BP.ColdPotato_BP_C"))
  (Variables|Default|SetCold%20Potato%20Ref _returnvalue))